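; Game mode Blueprint with helpers for spawning local players in a 2D side-scroller, currently inactive because BeginPlay is empty and the helper calls are unwired.
; GetPlayerStartPoints stores and prints all PlayerStart actors, but SpawnPlayers does not use them.
; SpawnPlayers loops to MaxPlayerCount, creating each local player, then spawning a BP_2DSideScrollerCharacter at the first TargetPoint found and possessing it with that player's controller.
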(event `self.ReceiveBeginPlay`)

(fn `GetPlayerStartPoints`
  (bind _outactors (`GameplayStatics.GetAllActorsOfClass` "/Script/Engine.PlayerStart"))
  (bind _output_get (set `self.PlayerStarts` _outactors))
  (for _array_element _output_get
    (`KismetSystemLibrary.PrintString` (`KismetSystemLibrary.GetDisplayName` _array_element) true true (struct :`G` 0.66 :`B` 1.0 :`A` 1.0) 222.0)))

(fn `SpawnPlayers`
  ;[1 1 1] Comment
  (for _index (range (`self.MaxPlayerCount`))
    (set `self.IndexPlayerSpawned` _index)
    (`KismetSystemLibrary.PrintString` "LOOP that spawns players" true true (struct :`G` 0.66 :`B` 1.0 :`A` 1.0) 222.0)
    (bind _outactors (`GameplayStatics.GetAllActorsOfClass` "/Script/Engine.TargetPoint"))
    ;;[1 1 1] empty slot for a player to inhabit,(it gives a player state player controller)
    (`GameplayStatics.CreatePlayer` (`self.IndexPlayerSpawned`))
    (bind _returnvalue (`|SpawnActorFromClass` "/Game/2DSideScrollerCPP/Blueprints/BP_2DSideScrollerCharacter.BP_2DSideScrollerCharacter_C" (`self.GetTransform` (`|GetArrayItem` _outactors)) "Undefined" "OverrideRootScale" null null))
    (`Controller.Possess` (`GameplayStatics.GetPlayerController` (`self.IndexPlayerSpawned`)) _returnvalue)))

(fn `UserConstructionScript`)